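; BP_DMG_Field is a damage area that periodically hurts overlapping Damageable actors.
; A looping one-second timer created paused at BeginPlay resumes on any overlap begin and pauses on any overlap end, even if other actors remain inside.
; Each tick of the timer applies fixed melee damage to overlapping Damageables with health left, spawning an explosion effect and sound at the field for each hit.
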(event `self.ReceiveBeginPlay`
  (bind _returnvalue (`KismetSystemLibrary.K2_SetTimer` null "Explode" 1.0 true true -1.0))
  (bind _output_get (set `self.ExplosionTimer` _returnvalue))
  (`KismetSystemLibrary.K2_PauseTimerHandle` _output_get))

(event `self.ReceiveActorBeginOverlap`
  (params (OtherActor :type "Actor Object Reference"))
  (`KismetSystemLibrary.K2_UnPauseTimerHandle` (`self.ExplosionTimer`)))

(event `self.ReceiveActorEndOverlap`
  (params (OtherActor :type "Actor Object Reference"))
  (`KismetSystemLibrary.K2_PauseTimerHandle` (`self.ExplosionTimer`)))

(event `Explode`
  (for _array_element (`self.GetOverlappingActors` null)
    (bind _asdamageable (cast `Damageable` _array_element))
    (bind _returnvalue (`Damageable.GetHealth` _asdamageable))
    (if (> _returnvalue 0.0)
      (`Damageable.Damage` _asdamageable (make `DamageInfo` 5.0 "Mele" "Hit"))
      (`self.PlayEffect`))))

(event `PlayEffect`
  (bind _returnvalue (`self.K2_GetActorLocation`))
  (`GameplayStatics.SpawnEmitterAtLocation` "/Game/StarterContent/Particles/P_Explosion.P_Explosion" _returnvalue (struct) (2.0 2.0 2.0))
  (`GameplayStatics.PlaySoundAtLocation` "/Game/StarterContent/Audio/Explosion01.Explosion01" _returnvalue (struct) 0.7 1.0 0.0 null null null null))

(fn `UserConstructionScript`)