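; NPC character with sword combat, a floating health bar and functions supplying health, patrol route, ideal ranges and movement speed.
; Montage notifies spawn the hand-socketed sword or destroy it, and montage endings fire callbacks for attack, equip and sheath.
; Damage defers to the parent and reveals the health bar while alive; Heal is a stub returning zero.
; The melee sphere-trace damage logic is disconnected, so attacks here deal no damage.
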(event `self.ReceiveBeginPlay`
  (bind _healthbar (`self.Healthbar`))
  (add `DamageSystemComponent.OnDeath` (`self.DamageSystem`) (`|CreateDelegate` :!event `HideHealthbar`))
  (bind _returnvalue (`|CreateWidget` "/Game/Modules/CharacterSystems/Widgets/WBP_FloatingHealthBar.WBP_FloatingHealthBar_C" null self))
  (`WidgetComponent.SetWidget` _healthbar _returnvalue)
  (`SceneComponent.SetVisibility` _healthbar false false))

(event `Attack`
  (bind _notifyname (`|PlayMontage` (`self.Mesh`) "/Game/EssentialAnimation/SwordShield/Animation/UE5/Sequence/SSH/Attack/Montage_SSH_Attack1.Montage_SSH_Attack1")
    (:`OnCompleted`
      (`self.OnAttackEnd` :!label _label))
    (:`OnInterrupted`
      (goto _label))
    (:`OnNotifyBegin`
      (switch `name` _notifyname))))

(event `EquipSword`
  (bind _notifyname (`|PlayMontage` (`self.Mesh`) "/Game/EssentialAnimation/SwordShield/Animation/UE5/Sequence/SSH/Equip/Montage_SSH_Unsheath_Hip.Montage_SSH_Unsheath_Hip")
    (:`OnCompleted`
      (`self.OnEquipSword`))
    (:`OnNotifyBegin`
      (switch `name` _notifyname
        (:`PickupSword`
          (bind _returnvalue (`|SpawnActorFromClass` "/Game/Modules/CharacterSystems/Weapons/BP_Sword.BP_Sword_C" (`self.GetTransform`) "Undefined" "MultiplyWithRoot" null null))
          (bind _output_get (set `self.SwordActor` _returnvalue))
          (bind _returnvalue_2 (`self.K2_AttachToComponent` _output_get (`self.Mesh`) "hand_rSocket" "SnapToTarget" "SnapToTarget" "SnapToTarget" true))
          (set `self.isWeaponEquiped` _returnvalue_2))))))

(event `SheathSword`
  (bind _notifyname (`|PlayMontage` (`self.Mesh`) "/Game/EssentialAnimation/SwordShield/Animation/UE5/Sequence/SSH/Equip/Montage_SSH_Sheath_Hip.Montage_SSH_Sheath_Hip")
    (:`OnCompleted`
      (`self.OnSheathSword`))
    (:`OnNotifyBegin`
      (switch `name` _notifyname
        (:`DropSword`
          (`self.K2_DestroyActor` (`self.SwordActor`))
          (set `self.isWeaponEquiped` false))))))

(fn `Damage`
  (params (DamageInfo :type "DamageInfo Structure"))
  (returns (ReturnValue :type "Float (single-precision)"))
  (bind _returnvalue (`parent.Damage` DamageInfo))
  (`|ExecutionSequence`
    (:`then_0`
      (if (not (`DamageSystemComponent.isDead` (`self.DamageSystem`)))
        (`SceneComponent.SetVisibility` (`self.Healthbar`) true false)))
    (:`then_1`
      (return _returnvalue))))

(fn `GetHealth`
  (returns (ReturnValue :type "Float (single-precision)"))
  (bind _returnvalue (`StatsComponent.GetBaseStat` (`self.Stats`) "health"))
  (return _returnvalue))

(fn `GetIdealRange`
  (returns (AttackRadius :type "Float (double-precision)") (DefendRadius :type "Float (double-precision)"))
  (return 200.0 350.0))

(fn `GetMaxHealth`
  (returns (ReturnValue :type "Float (single-precision)"))
  (bind _returnvalue (`StatsComponent.GetDerivedStat` (`self.Stats`) "max_health"))
  (return _returnvalue))

(fn `GetPatrolRoute`
  (returns (PatrolRoute :type "/Game/Modules/CharacterSystems/AI/BP_PatrolRoute Object Reference"))
  (return (`self.PatrolRoute`)))

(fn `Heal`
  (params (Amount :type "Float (single-precision)"))
  (returns (ReturnValue :type "Float (single-precision)"))
  (return 0.0))

(fn `HideHealthbar`
  (`SceneComponent.SetVisibility` (`self.Healthbar`) false false))

(fn `SetMovementSpeed`
  (params (Speed :type "ECharacterMovementSpeed Enum" :default "Idle"))
  (returns (`Speed Value` :type "Float (double-precision)"))
  (bind _output_get (set `CharacterMovementComponent.MaxWalkSpeed` (select `ECharacterMovementSpeed` Speed :`Walk` 100.0 :`Jog` 300.0 :`Sprint` 500.0 :!type "Float (single-precision)") (`self.CharacterMovement`)))
  (return _output_get))

(fn `UserConstructionScript`
  (`parent.UserConstructionScript`))