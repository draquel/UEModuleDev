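; BP_PatrolRoute is an actor that defines an AI patrol path with a spline component.
; It tracks a current point index and a direction, and IncrementPatrolRoute steps the index, flipping direction at the first and last spline points for back-and-forth movement.
; GetPointLocation returns the world-space location of the current spline point.
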(event `IncrementPatrolRoute`
  (bind _output_get (set `self.PatrolPointIndex` (+ (`self.PatrolPointIndex`) (`self.Direction`))))
  (if (== _output_get (- (`SplineComponent.GetNumberOfSplinePoints` (`self.PatrolRoute`)) 1))
    (set `self.Direction` -1)
    (elif (== (`self.PatrolPointIndex`) 0)
      (set `self.Direction` 1))))

(fn `GetPointLocation`
  (returns (Location :type "Vector Structure"))
  (return (`SplineComponent.GetLocationAtSplinePoint` (`self.PatrolRoute`) (`self.PatrolPointIndex`) "World")))

(fn `UserConstructionScript`)